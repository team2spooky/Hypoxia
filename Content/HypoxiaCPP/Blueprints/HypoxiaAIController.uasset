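; Monster AI controller for Hypoxia that starts the monster's behavior on BeginPlay.
; It initializes MonsterAIBlackboard and runs the MonsterAITree behavior tree, which drives all decisions.
; Tick is empty, and leftover unconnected nodes for setting a random WanderLocation and printing debug text never execute.
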(event EventBeginPlay
  (Class|AIController|UseBlackboard "/Game/HypoxiaCPP/AI/MonsterAIBlackboard.MonsterAIBlackboard")
  (AI|RunBehaviorTree "/Game/HypoxiaCPP/AI/MonsterAITree.MonsterAITree"))

(event EventTick
  (params (DeltaSeconds :type Float%20%28single-precision%29)))

(fn ConstructionScript)